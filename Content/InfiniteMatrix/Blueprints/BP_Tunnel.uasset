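; Endless tunnel segment with a rotating holed wall, an optional health pickup and spawned enemies.
; BeginPlay randomly places or removes the pickup; RandomizeWall and RandomizeEnemies, not called here, vary hole mesh, roll and enemy positions.
; The player's trigger overlap spawns the next tunnel and clears enemies, adding score, speed and self-destructing only without a wall hit.
; Wall hits cost player health, pickup hits restore it, and both destroy projectiles.
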(event `self.ReceiveBeginPlay`
  (`self.RandomizeHealth`))

(event `self.ReceiveTick`
  (params (DeltaSeconds :type "Float (single-precision)"))
  (`SceneComponent.K2_AddLocalRotation` (`self.WallMesh`) (`KismetMathLibrary.MakeRotator` (* DeltaSeconds (`self.RotateSpeed`))) false false))

(event `self.TriggerZone.OnComponentBeginOverlap`
  (params (OverlappedComponent :type "PrimitiveComponent Object Reference") (OtherActor :type "Actor Object Reference") (OtherComp :type "PrimitiveComponent Object Reference") (OtherBodyIndex :type Integer) (bFromSweep :type Boolean) (SweepResult :type "HitResult Structure (by ref)"))
  (bind _asbp_player (cast `/Game/InfiniteMatrix/Blueprints/BP_Player` OtherActor))
  (`/Game/InfiniteMatrix/Blueprints/BP_TunnelSpawner. SpawnTunnelAtSpawnPoint` (`self.TunnelSpawner`))
  (for _array_element (`self.Enemies`)
    (`/Engine/EditorBlueprintResources/StandardMacros.IsValid` _array_element
      (:`Is Valid`
        (`self.K2_DestroyActor` _array_element))))
  (if (not (`self.Hit`))
    (`/Game/InfiniteMatrix/Blueprints/BP_Player.IncrementScore` _asbp_player true 100)
    (`/Game/InfiniteMatrix/Blueprints/BP_Player.IncrementSpeed` _asbp_player)
    (`self.K2_DestroyActor`)))

(event `self.WallMesh.OnComponentHit`
  (params (HitComponent :type "PrimitiveComponent Object Reference") (OtherActor :type "Actor Object Reference") (OtherComp :type "PrimitiveComponent Object Reference") (NormalImpulse :type "Vector Structure") (Hit :type "HitResult Structure (by ref)"))
  (bind _asbp_player (cast `/Game/InfiniteMatrix/Blueprints/BP_Player` OtherActor)
    (:`then`
      (`/Game/InfiniteMatrix/Blueprints/BP_Player.DecreaseHealth` _asbp_player)
      (`PrimitiveComponent.SetCollisionEnabled` HitComponent "NoCollision")
      (set `self.Hit` true))
    (:`CastFailed`
      (bind _asbp_projectile (cast `/Game/InfiniteMatrix/Blueprints/BP_Projectile` OtherActor))
      (`self.K2_DestroyActor` _asbp_projectile))))

(event `self.Health.OnComponentHit`
  (params (HitComponent :type "PrimitiveComponent Object Reference") (OtherActor :type "Actor Object Reference") (OtherComp :type "PrimitiveComponent Object Reference") (NormalImpulse :type "Vector Structure") (Hit :type "HitResult Structure (by ref)"))
  (bind _asbp_player (cast `/Game/InfiniteMatrix/Blueprints/BP_Player` OtherActor)
    (:`then`
      (`/Game/InfiniteMatrix/Blueprints/BP_Player.Increase Health` _asbp_player)
      (`ActorComponent.K2_DestroyComponent` HitComponent))
    (:`CastFailed`
      (bind _asbp_projectile (cast `/Game/InfiniteMatrix/Blueprints/BP_Projectile` OtherActor))
      (`self.K2_DestroyActor` _asbp_projectile))))

(fn `RandomizeEnemies`
  (params (NumEnemies :type Integer))
  (bind _returnvalue (`SceneComponent.K2_GetComponentToWorld` (`self.SpawnPoint`)))
  (for _ (range 1 (+ NumEnemies 1))
    (bind _returnvalue_2 (`|SpawnActorFromClass` "/Game/InfiniteMatrix/Blueprints/BP_Enemy.BP_Enemy_C" (`KismetMathLibrary.MakeTransform` (`KismetMathLibrary.MakeVector` (+ (`KismetMathLibrary.RandomFloatInRange` -2000.0 -500.0) (.x (.location _returnvalue))) (+ (.y (.location _returnvalue)) (`KismetMathLibrary.RandomFloatInRange` -300.0 300.0)) (+ (.z (.location _returnvalue)) (`KismetMathLibrary.RandomFloatInRange` -300.0 300.0))) (.rotation _returnvalue) (1.0 1.0 2.0)) "AdjustIfPossibleButAlwaysSpawn" "MultiplyWithRoot" null null))
    (`KismetArrayLibrary.Array_Add` (`self.Enemies`) _returnvalue_2)))

(fn `RandomizeHealth`
  (if (<= (`KismetMathLibrary.RandomFloat`) 0.3)
    (`SceneComponent.K2_SetRelativeLocation` (`self.Health`) (`KismetMathLibrary.MakeVector` 1235.0 (`KismetMathLibrary.RandomFloatInRange` -200.0 200.0) (`KismetMathLibrary.RandomFloatInRange` -200.0 200.0)) false true)
    (else
      (`ActorComponent.K2_DestroyComponent` (`self.Health`)))))

(fn `RandomizeWall`
  (`StaticMeshComponent.SetStaticMesh` (`self.WallMesh`) (select `int` (`KismetMathLibrary.RandomIntegerInRange` 0 3) :`0` "/Game/InfiniteMatrix/Meshes/SM_Hole_01.SM_Hole_01" :`1` "/Game/InfiniteMatrix/Meshes/SM_Hole_02.SM_Hole_02" :`2` "/Game/InfiniteMatrix/Meshes/SM_Hole_03.SM_Hole_03" :`3` "/Game/InfiniteMatrix/Meshes/SM_Hole_04.SM_Hole_04" :!type "StaticMesh Object Reference"))
  (`SceneComponent.K2_AddLocalRotation` (`self.WallMesh`) (`KismetMathLibrary.MakeRotator` (`KismetMathLibrary.RandomFloatInRange` 0.0 360.0)) false false))

(fn `UserConstructionScript`)